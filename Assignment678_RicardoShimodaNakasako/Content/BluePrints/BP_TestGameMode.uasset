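; Test game mode that spawns AI enemy bots at locations chosen by an Environment Query.
; SpawnNewBot runs EQS_FindSpawnLocation in random best-25% mode and hands the finished query to SpawnBot.
; On success, SpawnBot draws a debug sphere and spawns a bot at each returned location.
; Its type switch covers rifle, shotgun and sniper AI, but the fixed random range always selects the default sniper.
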(event `self.SpawnNewBot`
  (bind _returnvalue (`EnvQueryManager.RunEQSQuery` "/Game/BluePrints/EQS_FindSpawnLocation.EQS_FindSpawnLocation" self "RandomBest25Pct"))
  (add `EnvQueryInstanceBlueprintWrapper.OnQueryFinishedEvent` _returnvalue (delegate `SpawnBot`)))

(event `SpawnBot`
  (params (QueryInstance :type "EnvQueryInstanceBlueprintWrapper Object Reference") (QueryStatus :type "EEnvQueryStatus Enum" :default "Processing"))
  (switch `EEnvQueryStatus` QueryStatus
    (:`Success`
      (bind _resultlocations (`EnvQueryInstanceBlueprintWrapper.GetQueryResultsAsLocations` QueryInstance))
      (for _array_element _resultlocations
        (`KismetSystemLibrary.DrawDebugSphere` _array_element 100.0 12 (struct :`R` 1.0 :`G` 0.419257 :`B` 0.06169 :`A` 1.0) 5.0 3.0)
        (switch `int` (`KismetMathLibrary.RandomIntegerInRange` 2 2)
          (:`Default`
            (bind _returnvalue (`KismetMathLibrary.MakeTransform` _array_element))
            (`|SpawnActorFromClass` "/Game/BluePrints/BP_SniperAI.BP_SniperAI_C" _returnvalue "Undefined" "OverrideRootScale" null null))
          (:`0`
            (`|SpawnActorFromClass` "/Game/BluePrints/BP_Rifle_AI.BP_Rifle_AI_C" _returnvalue "Undefined" "OverrideRootScale" null null))
          (:`1`
            (`|SpawnActorFromClass` "/Game/BluePrints/BP_Shotgun_AI.BP_Shotgun_AI_C" _returnvalue "Undefined" "OverrideRootScale" null null)))))))

(fn `UserConstructionScript`)